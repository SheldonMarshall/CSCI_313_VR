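; Crystal base for the statue minigame that detects when blue, green and red crystals all sit on their pedestals.
; On overlap, each color's collider casts to GrabableCrystal_B, drops and snaps the crystal to its slot, and stores its mesh.
; Tick checks all three overlaps, runs CanOpen with button and welding minigames hardcoded true, and sends the crystal key state to Level_Hopper_S2F via GatewayMessage.
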(event `self.ReceiveTick`
  (params (DeltaSeconds :type "Float (single-precision)"))
  (bind _returnvalue (and (`PrimitiveComponent.IsOverlappingComponent` (`self.Blue_BC`) (`self.Static Mesh_B`)) (`PrimitiveComponent.IsOverlappingComponent` (`self.Green_BC`) (`self.Static Mesh_G`)) (`PrimitiveComponent.IsOverlappingComponent` (`self.Red_BC`) (`self.Static Mesh_R`))))
  (if _returnvalue
    (bind _can_open (`self.CanOpen?` _returnvalue true true))
    (if _can_open
      (bind _output_get (set `self.B_CrystalKey` true))
      (bind _returnvalue_2 (`GameplayStatics.GetActorOfClass` "/Game/My_Assets/BluePrints/Level_Changes/Level_Hopper_S2F.Level_Hopper_S2F_C"))
      (bind _output_get_2 (set `self.Actor` _returnvalue_2))
      (message `/Game/My_Assets/BluePrints/Interfaces/BI_PassThourgh.Gateway` _output_get_2 _output_get)
      (`KismetSystemLibrary.PrintString` "True")
      (else
        (bind _output_get_3 (set `self.B_CrystalKey` false))
        (bind _returnvalue_3 (`GameplayStatics.GetActorOfClass` "/Game/My_Assets/BluePrints/Level_Changes/Level_Hopper_S2F.Level_Hopper_S2F_C"))
        (bind _output_get_4 (set `self.Actor` _returnvalue_3))
        (message `/Game/My_Assets/BluePrints/Interfaces/BI_PassThourgh.Gateway` _output_get_4 _output_get_3)
        (`KismetSystemLibrary.PrintString` "False")))))

(event `self.Blue_BC.OnComponentBeginOverlap`
  (params (OverlappedComponent :type "PrimitiveComponent Object Reference") (OtherActor :type "Actor Object Reference") (OtherComp :type "PrimitiveComponent Object Reference") (OtherBodyIndex :type Integer) (bFromSweep :type Boolean) (SweepResult :type "HitResult Structure (by ref)"))
  ;[1 1 1] Blue
  (bind _staticmesh (`self.Attached` (`self.StatueBase_Blue_Mid`) OtherActor))
  (set `self.Static Mesh_B` _staticmesh))

(event `self.Green_BC.OnComponentBeginOverlap`
  (params (OverlappedComponent :type "PrimitiveComponent Object Reference") (OtherActor :type "Actor Object Reference") (OtherComp :type "PrimitiveComponent Object Reference") (OtherBodyIndex :type Integer) (bFromSweep :type Boolean) (SweepResult :type "HitResult Structure (by ref)"))
  ;[1 1 1] Green
  (bind _staticmesh (`self.Attached` (`self.StatueBase_Green_Mid`) OtherActor))
  (set `self.Static Mesh_G` _staticmesh))

(event `self.Red_BC.OnComponentBeginOverlap`
  (params (OverlappedComponent :type "PrimitiveComponent Object Reference") (OtherActor :type "Actor Object Reference") (OtherComp :type "PrimitiveComponent Object Reference") (OtherBodyIndex :type Integer) (bFromSweep :type Boolean) (SweepResult :type "HitResult Structure (by ref)"))
  ;[1 1 1] Red
  (bind _staticmesh (`self.Attached` (`self.StatueBase_Red_Mid`) OtherActor))
  (set `self.Static Mesh_R` _staticmesh))

(fn `CanOpen?`
  (params (Statue_MiniGame :type Boolean) (Button_MiniGame :type Boolean) (Welding_MiniGame :type Boolean))
  (returns (Can_Open :type Boolean))
  (return (and Statue_MiniGame Button_MiniGame Welding_MiniGame)))

(fn `PassThrough`
  (params (Input :type String))
  (return))

(fn `UserConstructionScript`)